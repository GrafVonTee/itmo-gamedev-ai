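; AI controller for the Pnevmoslon bot that starts its behavior tree and feeds it the bot's hunt points.
; On possess it runs BT_Pnevmoslon, then InitializePoints casts the controlled pawn to BP_Pnevmoslon.
; It copies the first four entries of the pawn's HuntedPointsArray into blackboard object keys FirstPoint through FourthPoint, with fixed indices and no length check.
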(event EventBeginPlay)

(event EventTick
  (params (DeltaSeconds :type Float%20%28single-precision%29)))

(event EventPossess
  (params (PossessedPawn :type Pawn%20Object%20Reference))
  (AI|RunBehaviorTree "/Game/Lab2/Boards/BT_Pnevmoslon.BT_Pnevmoslon")
  (CallFunction|InitializePoints))

(fn ConstructionScript)

(fn InitializePoints
  (bind _asbp_pnevmoslon (Utilities|Casting|CastToBP_Pnevmoslon (Pawn|GetControlledPawn)))
  (bind _output_get (Variables|Default|SetTargetPoint_1 (Utilities|Array|Get(acopy) (Variables|/Game/Lab2/Bots/BP_Pnevmoslon.BP_Pnevmoslon_C|GetHuntedPointsArray _asbp_pnevmoslon))))
  (AI|Components|Blackboard|SetValueasObject (AI|GetBlackboard 0) (Utilities|String|StringToName "FirstPoint") _output_get)
  (bind _output_get_2 (Variables|Default|SetTargetPoint_2 (Utilities|Array|Get(acopy) (Variables|/Game/Lab2/Bots/BP_Pnevmoslon.BP_Pnevmoslon_C|GetHuntedPointsArray _asbp_pnevmoslon) 1)))
  (AI|Components|Blackboard|SetValueasObject (AI|GetBlackboard 0) (Utilities|String|StringToName "SecondPoint") _output_get_2)
  (bind _output_get_3 (Variables|Default|SetTargetPoint_3 (Utilities|Array|Get(acopy) (Variables|/Game/Lab2/Bots/BP_Pnevmoslon.BP_Pnevmoslon_C|GetHuntedPointsArray _asbp_pnevmoslon) 2)))
  (AI|Components|Blackboard|SetValueasObject (AI|GetBlackboard 0) (Utilities|String|StringToName "ThirdPoint") _output_get_3)
  (bind _output_get_4 (Variables|Default|SetTargetPoint_4 (Utilities|Array|Get(acopy) (Variables|/Game/Lab2/Bots/BP_Pnevmoslon.BP_Pnevmoslon_C|GetHuntedPointsArray _asbp_pnevmoslon) 3)))
  (AI|Components|Blackboard|SetValueasObject (AI|GetBlackboard 0) (Utilities|String|StringToName "FourthPoint") _output_get_4))