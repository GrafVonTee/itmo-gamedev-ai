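; AI controller that steers its pawn, a cube, along walls on its right-hand side.
; Each tick it line traces forward and 45 degrees right, ignoring Characters, to pick a movement direction fed to AddMovementInput.
; It turns away from blocked paths, goes straight beside a right wall, and rotates when both traces miss.
; A rotation counter makes it go straight after a full turn without hits.
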(event EventBeginPlay)

(event EventTick
  (params (DeltaSeconds :type Float%20%28single-precision%29))
  (bind _returnvalue (Pawn|GetControlledPawn))
  (bind _returnvalue_2 (Pawn|GetControlledPawn))
  (bind _rotationdegreebyz (Variables|Default|GetRotationDegreeByZ))
  (bind _results (Variables|Default|GetResults))
  (bind _returnvalue_3 (Transformation|GetActorLocation _returnvalue_2))
  (bind _returnvalue_4 (Transformation|GetActorForwardVector _returnvalue_2))
  (bind _returnvalue_5 (Transformation|GetActorForwardVector _returnvalue))
  (bind _outactors (Actor|GetAllActorsOfClass "/Script/Engine.Character"))
  (for _array_element (Utilities|Array|MakeArray _returnvalue_4 (Math|Vector|RotateVector _returnvalue_4 "0,45.000000, 0"))
    (bind _returnvalue_6 (Collision|LineTraceByChannel _returnvalue_3 (+ (* _array_element (Variables|Default|GetSightLen)) _returnvalue_3) "TraceTypeQuery1" false _outactors "ForOneFrame"))
    (Utilities|Array|Add (Variables|Default|GetResults) _returnvalue_6))
  (Utilities|FlowControl|Sequence
    (:then_0
      ;[1 1 1] Check the wall is in front of pawn
      (if (Utilities|Array|Get(acopy) _results)
        ;[1 1 1] If so, check the wall is on the right-hand side for strong rotation
        (if (Utilities|Array|Get(acopy) _results 1)
          (Variables|Default|SetMovementDirection (Math|Vector|RotateVector _returnvalue_5 "0,-10.000000, 0"))
          (else
            (Variables|Default|SetMovementDirection (Math|Vector|RotateVector _returnvalue_5 "0,10.000000, 0"))))
        ;[1 1 1] Make counter Zero if the cube is not rotating
        (Variables|Default|SetRotationCounter 0.0 :!label _label)
        (else
          ;[1 1 1] If not, then try to steak to the right wall
          (if (Utilities|Array|Get(acopy) _results 1)
            (Variables|Default|SetMovementDirection _returnvalue_5)
            (goto _label)
            (else
              ;[1 1 1] Check the cube is nor rotating too much
              (Variables|Default|SetRotationCounter (+ (Variables|Default|GetRotationCounter) _rotationdegreebyz))
              (if (>= (Variables|Default|GetRotationCounter) 3.6e+02)
                (Variables|Default|SetMovementDirection _returnvalue_5)
                (else
                  (Variables|Default|SetMovementDirection (Math|Vector|RotateVector _returnvalue_5 (Math|Rotator|MakeRotator 0.0 0.0 _rotationdegreebyz))))))))))
    (:then_1
      (Pawn|Input|AddMovementInput _returnvalue (Variables|Default|GetMovementDirection) (* (Variables|Default|GetSpeed) DeltaSeconds) false)
      (Utilities|Array|Clear _results))))

(fn ConstructionScript)