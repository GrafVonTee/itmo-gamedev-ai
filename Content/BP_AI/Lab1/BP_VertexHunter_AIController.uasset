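; AI controller that sends a BP_VertexHunter pawn around a looping patrol of its hunting points.
; On BeginPlay it casts the controlled pawn and copies its HuntingPoints array.
; MoveToNextPoint runs AI MoveTo toward the current point, then on success advances the index, wraps it at the array's end and calls itself again.
; A failed move has no handler, so the patrol does not continue after one.
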(event Custom|MoveToNextPoint
  (AI|AIMoveTo 0 "0, 0, 0" (Utilities|Array|Get(acopy) (Variables|Default|GetHuntingPoints) (Variables|Default|GetCurrent%20Index)) 5.0 false
    (:OnSuccess
      (bind _result (Math|Integer|IncrementInt (Variables|Default|GetCurrent%20Index))
        (:%20%20
          (if (== _result (Utilities|Array|Length (Variables|Default|GetHuntingPoints)))
            (Variables|Default|SetCurrent%20Index 0))
          (CallFunction|MovetoNextPoint))))))

(event EventBeginPlay
  (bind _asbp_vertex_hunter (Utilities|Casting|CastToBP_VertexHunter (Pawn|GetControlledPawn)))
  (Variables|Default|SetHuntingPoints (Variables|/Game/BP_AI/Lab1/BP_VertexHunter.BP_VertexHunter_C|GetHuntingPoints _asbp_vertex_hunter))
  (CallFunction|MovetoNextPoint))

(fn ConstructionScript)